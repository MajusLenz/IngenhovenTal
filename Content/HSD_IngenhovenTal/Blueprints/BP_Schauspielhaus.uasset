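; Schauspielhaus building actor whose three grass-roof layers (top, podest, underside) can lift off, hover and land.
; A looping hover timeline, driven from Tick, moves each layer from a shared hover position by a differently scaled share of the construction-script offset.
; Abheben (lift off) and Landen (land) timelines set AnimationAlpha, which blends the layers between zero relative location and the hover motion.
; BeginPlay saves original relative locations, but the animation does not use them.
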(event `self.ReceiveBeginPlay`
  (`self.SetSavedRelativeLocations`))

(event `self.ReceiveTick`
  (params (DeltaSeconds :type "Float (single-precision)"))
  (bind _hoverpositionvector (`self.HoverPositionVector`))
  ;[0.5147 0 1] Hovern
  (bind (_direction _alpha) (`Timeline|TL_Hover` :!label _label)
    (:`Update`
      (bind (_topanim _middleanim _loweranim) (`self.AnimateRelativeLocations` _alpha _hoverpositionvector _hoverpositionvector _hoverpositionvector (`self.HoverOffsetVector`)))
      (`self.BlendBetweenAnimationAndStatic` _topanim _middleanim _loweranim (`self.AnimationAlpha`)))
    (:`Finished`
      (goto _label :!via `PlayFromStart`))))

(event `Abheben`
  ;[1 0.55 0] Abheben
  (bind (_direction _alpha) (`Timeline|TL_Abheben` :!via `PlayFromStart`)
    (:`Update`
      (set `self.AnimationAlpha` _alpha))))

(event `Landen`
  ;[0 1 0.11] Landen
  (bind (_direction _alpha) (`Timeline|TL_Landen` :!via `PlayFromStart`)
    (:`Update`
      (set `self.AnimationAlpha` _alpha))))

(fn `AnimateRelativeLocations`
  (params (Alpha :type "Float (single-precision)") (Top :type "Vector Structure") (Middle :type "Vector Structure") (Lower :type "Vector Structure") (AnimionOffset :type "Vector Structure"))
  (returns (TopAnim :type "Vector Structure") (MiddleAnim :type "Vector Structure") (LowerAnim :type "Vector Structure"))
  (return (`KismetMathLibrary.VLerp` Top (- Top (* AnimionOffset (0.8 0.8 0.8))) Alpha) (`KismetMathLibrary.VLerp` Middle (- Middle (* AnimionOffset (0.6 0.6 0.6))) Alpha) (`KismetMathLibrary.VLerp` Lower (- Lower (* AnimionOffset (0.4 0.4 0.4))) Alpha)))

(fn `BlendBetweenAnimationAndStatic`
  (params (AnimTop :type "Vector Structure") (AnimMiddle :type "Vector Structure") (AnimLower :type "Vector Structure") (Alpha :type "Float (double-precision)"))
  (`SceneComponent.K2_SetRelativeLocation` (`self.Schauspielhaus_GrasDach_Dach_Top`) (`KismetMathLibrary.VLerp` (0.0 0.0 0.0) AnimTop Alpha) false false)
  (`SceneComponent.K2_SetRelativeLocation` (`self.Schauspielhaus_GrasDach_Dach_Podest`) (`KismetMathLibrary.VLerp` (0.0 0.0 0.0) AnimMiddle Alpha) false false)
  (`SceneComponent.K2_SetRelativeLocation` (`self.Schauspielhaus_GrasDach_Dach_Unterseite`) (`KismetMathLibrary.VLerp` (0.0 0.0 0.0) AnimLower Alpha) false false))

(fn `getSavedRelativeLocations`
  (returns (Top :type "Vector Structure") (Middle :type "Vector Structure") (Lower :type "Vector Structure"))
  (return (`self.TopRelativeLocation`) (`self.MiddleRelativeLocation`) (`self.LowerRelativeLocation`)))

(fn `SetSavedRelativeLocations`
  (set `self.TopRelativeLocation` (`SceneComponent.RelativeLocation` (`self.Schauspielhaus_GrasDach_Dach_Top`)))
  (set `self.MiddleRelativeLocation` (`SceneComponent.RelativeLocation` (`self.Schauspielhaus_GrasDach_Dach_Podest`)))
  (set `self.LowerRelativeLocation` (`SceneComponent.RelativeLocation` (`self.Schauspielhaus_GrasDach_Dach_Unterseite`)))
  (return))

(fn `UserConstructionScript`
  (set `self.HoverOffsetVector` (`KismetMathLibrary.MakeVector` (`self.X`) (`self.Y`) (`self.Z`)))
  (`TimelineComponent.SetPlayRate` (`self.TL_Hover`) (`self.HoverSpeed`)))